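; Player controller for a puzzle game that manages the player's cursor mode: open, flag or question.
; ChangeNextCursor cycles through the three modes in that order, but only when the UseHelpIcon game option is on.
; Each switch updates PlayerCursor and calls ChangeUiCursor, which forwards the new mode to ScrollReference through ChangeCursorMessage when that reference is set.
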(event `ChangeNextCursor`
  (bind (_gameoptions_difficulty _gameoptions_rowsize _gameoptions_colsize _gameoptions_numbombs _gameoptions_timelimit _gameoptions_usetimelimit _gameoptions_usehelpicon) (break `GameOptions` (`self.GameOptions`)))
  (if _gameoptions_usehelpicon
    (switch `EPlayerCursor` (`self.PlayerCursor`)
      (:`OPEN`
        (`self.SetPlayerCursor` "FLAG")
        (`self.ChangeUiCursor` "FLAG"))
      (:`FLAG`
        (`self.SetPlayerCursor` "QUEST")
        (`self.ChangeUiCursor` "QUEST"))
      (:`QUEST`
        (`self.SetPlayerCursor` "OPEN")
        (`self.ChangeUiCursor` "OPEN")))))

(event `ChangeUiCursor`
  (params (PlayerCursor :type "EPlayerCursor Enum" :default "OPEN"))
  (bind _scrollreference (`self.ScrollReference`))
  (if (!= _scrollreference null)
    (message `/Game/BluePrints/BPI_Interact.ChangeCursor ` _scrollreference PlayerCursor)))

(fn `UserConstructionScript`)