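; Directional light actor for the puzzle game that dims or lights the level according to the Dark Mode setting.
; On BeginPlay it reads BP_PuzzleProjGameInstance, taking Dark Mode from the game options in Simple Mode and from the level options otherwise.
; Dark Mode sets the light to near-zero intensity, while normal mode applies a fixed brighter intensity.
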(event `self.ReceiveBeginPlay`
  (bind _asbp_puzzle_proj_game_instance (cast `/Game/BluePrints/BP_PuzzleProjGameInstance` (`GameplayStatics.GetGameInstance`)))
  (if (`PuzzleProjGameInstance.isSimpleModeOn` _asbp_puzzle_proj_game_instance)
    (if (`.DarkMode` (break `GameOptions` (`PuzzleProjGameInstance.GameOptions` _asbp_puzzle_proj_game_instance)))
      (`LightComponent.SetIntensity` (`self.LightComponent`) 0.001 :!label _label)
      (else
        (`LightComponent.SetIntensity` (`self.LightComponent`) 1.72 :!label _label_2)))
    (else
      (bind _returnvalue (`PuzzleProjGameInstance.GetLevelOptions` _asbp_puzzle_proj_game_instance))
      (if (`.DarkMode` (break `GameOptions` _returnvalue))
        (goto _label)
        (else
          (goto _label_2))))))

(fn `UserConstructionScript`)